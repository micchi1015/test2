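; BP_Enemy is an enemy that cycles between waiting and timed shooting at the first-person player, and opens the Result level when defeated.
; Tick timers start and end each attack, during which it turns toward the player and spawns EnemyBullet projectiles at intervals.
; Bullet hits on its sphere play a sound and reduce clamped health, updating a percentage.
; BeginPlay hands the enemy reference to its BP_EnemyLife widget for the life bar.
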(event `self.ReceiveBeginPlay`
  ;[1 1 1] Enemyのライフバーを常に表示
  (bind _asbp_enemy_life (cast `/Game/BlueParint/BP_EnemyLife` (`WidgetComponent.GetUserWidgetObject` (`self.EnemyLife`))))
  (set `/Game/BlueParint/BP_EnemyLife.BP_Enemy3` self _asbp_enemy_life))

(event `self.Sphere0.OnComponentHit`
  (params (HitComponent :type "PrimitiveComponent Object Reference") (OtherActor :type "Actor Object Reference") (OtherComp :type "PrimitiveComponent Object Reference") (NormalImpulse :type "Vector Structure") (Hit :type "HitResult Structure (by ref)"))
  ;[1 1 1] CollisionにBulletが当たったらダメージ追加
  (cast `Bullet` OtherActor)
  (`self.Take Damage` 10.0)
  (`GameplayStatics.PlaySound2D` "/Game/Sound/SE_Hit.SE_Hit" 1.0 1.0 0.0 null null)
  ;[1 1 1] EnemyのLifeが0になったらResultにいく
  (if (<= (`self.MAX_LIFE`) 0.0)
    (`GameplayStatics.OpenLevelBySoftObjectPtr` "/Game/Maps/Result.Result")))

(event `self.ReceiveTick`
  (params (DeltaSeconds :type "Float (single-precision)"))
  (if (not (`self.IsAtacck`))
    (`|ExecutionSequence`
      (:`then_1`
        (set `self.ElapsedTime_LastAttack` (+ DeltaSeconds (`self.ElapsedTime_LastAttack`)))
        (if (>= (`self.ElapsedTime_LastAttack`) (`self.AttackInterval`))
          (`self.StartAttck`))))
    (else
      (bind _target (`self.Target`)
        (:`then`
          (`|ExecutionSequence`
            (:`then_0`
              (`self.K2_SetActorRotation` (`KismetMathLibrary.FindLookAtRotation` (`self.K2_GetActorLocation`) (+ (`self.K2_GetActorLocation` _target) (`KismetMathLibrary.MakeVector` 0.0 0.0 (`CapsuleComponent.GetScaledCapsuleHalfHeight` (`Character.CapsuleComponent` _target))))))
              (set `self.ElapsedTime_AttackStart` (+ DeltaSeconds (`self.ElapsedTime_AttackStart`)))
              (set `self.ElapsedTime_LastShot` (+ DeltaSeconds (`self.ElapsedTime_LastShot`))))
            (:`then_1`
              (if (>= (`self.ElapsedTime_LastShot`) (`self.ShotInterval`))
                (`self.SpawnProjectile`)))
            (:`then_2`
              (if (>= (`self.ElapsedTime_AttackStart`) (`self.AttackEndTime`))
                (`self.EndAtacck`)))))
        (:`else`)))))

(fn `EndAtacck`
  (set `self.IsAtacck` false))

(fn `SpawnProjectile`
  (bind (_returnvalue_location _returnvalue_rotation _returnvalue_scale) (`KismetMathLibrary.BreakTransform` (`self.GetTransform`)))
  (`|SpawnActorFromClass` "/Script/FPS.EnemyBullet" (`KismetMathLibrary.MakeTransform` (+ _returnvalue_location (* (`SceneComponent.GetForwardVector` (`self.CapsuleComponent`)) 100.0)) _returnvalue_rotation _returnvalue_scale) "Undefined" "OverrideRootScale" null null)
  (set `self.ElapsedTime_LastShot` 0.0))

(fn `StartAttck`
  (locals (NewLocalVar_0 :type "/Game/BlueParint/BP_FPSCharacter Object Reference"))
  (set `self.IsAtacck` true)
  (set `self.ElapsedTime_LastAttack` 0.0)
  (set `self.ElapsedTime_AttackStart` 0.0)
  (set `self.ElapsedTime_LastShot` 0.0)
  (`self.Target`
    (:`then`)
    (:`else`
      (bind _outactors (`GameplayStatics.GetAllActorsOfClass` "/Game/BlueParint/BP_FPSCharacter.BP_FPSCharacter_C"))
      (set `self.Target` (`|GetArrayItem` _outactors)))))

(fn `Take Damage`
  (params (Damage :type "Float (double-precision)"))
  (bind _output_get (set `self.MAX_LIFE` (`KismetMathLibrary.FClamp` (- (`self.MAX_LIFE`) Damage) 0.0 500.0)))
  (set `self.LIFE_PERCENTAGE` (/ _output_get 500.0)))

(fn `UserConstructionScript`)