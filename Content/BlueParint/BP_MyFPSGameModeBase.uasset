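; BP_MyFPSGameModeBase is an FPS game mode that runs a timed round and restarts players when they die.
; BeginPlay binds the player-died event, resets the clock and shows the BP_Time widget.
; Tick first counts down a pre-start Timer through a one-second Delay, then sets Start once via DoOnce.
; After that, Tick drains CurrentTime and opens the GameOver level when it drops below zero.
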(event `self.ReceiveBeginPlay`
  (add `self.OnPlayerDied` (delegate `PlayerDied`))
  (bind _output_get (set `self.MAX_TIME` 20.0))
  (set `self.CurrentTime` _output_get)
  (bind _returnvalue (`|CreateWidget` "/Game/BlueParint/BP_Time.BP_Time_C"))
  (bind _output_get_2 (set `self.UITime` _returnvalue))
  (`UserWidget.AddToViewport` _output_get_2 0))

(event `PlayerDied` :!signature `self.OnPlayerDied`
  (params (Character :type "Character Object Reference"))
  (`self.RestartPlayer` (`Pawn.GetController` Character)))

(event `self.ReceiveTick`
  (params (DeltaSeconds :type "Float (single-precision)"))
  (if (`self.Start`)
    (set `self.CurrentTime` (- (`self.CurrentTime`) DeltaSeconds))
    (if (< (`self.CurrentTime`) 0.0)
      (`GameplayStatics.OpenLevelBySoftObjectPtr` "/Game/Maps/GameOver.GameOver"))
    (elif (<= (`self.Timer`) 0)
      (`/Engine/EditorBlueprintResources/StandardMacros.DoOnce` false
        (:`Completed`
          (`self.Starttimer`)))
      (else
        (`KismetSystemLibrary.Delay` 1.0)
        (set `self.Timer` (- (`self.Timer`) 1))))))

(event `Starttimer`
  (set `self.Start` true))

(fn `UserConstructionScript`)